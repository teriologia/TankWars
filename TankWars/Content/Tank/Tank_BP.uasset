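; Tank pawn Blueprint that wires up the tank's components and player input for aiming, driving and firing.
; BeginPlay passes the barrel and turret references and initialises TankMovement with both tracks.
; Axis inputs rotate the azimuth gimbal and spring arm to aim the camera, set each track's throttle directly or send forward intent to TankMovement.
; The Fire action calls TankFire.
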(event EventBeginPlay
  (Class|Tank|SetBarrelRefferance (Variables|Default|GetBarrel))
  (Class|Tank|SetTurretRefferance (Variables|Default|GetTurret))
  (Class|TankMovementComponent|Initialise (Variables|Default|GetTankMovement) (Variables|Default|GetTrack_L) (Variables|Default|GetTrack_R)))

(event Input|ActionEvents|InputActionFire
  (params (Key :type Key%20Structure))
  ;[1 1 1] Fire
  (:Pressed
    (Class|Tank|TankFire)))

(event Input|AxisEvents|InputAxisAimAzimuth
  (params (AxisValue :type Float%20%28single-precision%29))
  ;[1 1 1] Camera settings
  (Transformation|AddLocalRotation (Variables|Default|GetAzimuth%20Gimbel) (Math|Rotator|MakeRotator 0.0 0.0 AxisValue) false false))

(event Input|AxisEvents|InputAxisAimElevation
  (params (AxisValue :type Float%20%28single-precision%29))
  ;[1 1 1] Camera settings
  (Transformation|AddLocalRotation (Variables|Default|GetSpringArm) (Math|Rotator|MakeRotator 0.0 AxisValue 0.0) false false))

(event Input|AxisEvents|InputAxisMoveForward
  (params (AxisValue :type Float%20%28single-precision%29))
  ;[1 1 1] Tank movement
  (Class|TankMovementComponent|IntendMoveForward (Variables|Default|GetTankMovement) AxisValue))

(event Input|AxisEvents|InputAxisLeftTrackThrottle
  (params (AxisValue :type Float%20%28single-precision%29))
  ;[1 1 1] Tank movement
  (Class|TankTack|SetThrottle (Variables|Default|GetTrack_L) AxisValue))

(event Input|AxisEvents|InputAxisRightTrackThrottle
  (params (AxisValue :type Float%20%28single-precision%29))
  ;[1 1 1] Tank movement
  (Class|TankTack|SetThrottle (Variables|Default|GetTrack_R) AxisValue))

(fn ConstructionScript)